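; Player-controlled pawn for a skipping stone: a physics mesh launched with a start impulse that the player boosts to skip across water.
; A downward sphere trace on a water profile measures distance to the surface each tick, printing it on screen.
; Boost input uses a curve of that distance, stronger near the surface, to add forward velocity and replace vertical velocity.
; Boosts are blocked while upward velocity exceeds a threshold.
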(event Input|EnhancedActionEvents|EnhancedInputActionIA_Boost
  (params (ActionValue :type Boolean) (ElapsedSeconds :type Float%20%28double-precision%29) (TriggeredSeconds :type Float%20%28double-precision%29) (InputAction :type Input%20Action%20Object%20Reference :default "/Game/SkippyStone/Input/IA_Boost.IA_Boost"))
  (:Triggered
    (Variables|Default|SetisBoosting true)
    (CallFunction|UpdateBoostingState)
    (if (not (Variables|Default|GetisBoosting))
      (CallFunction|Boost (stale EventTick _distancebelow) (Variables|Default|GetForwardBoostStrength) (Variables|Default|GetUpBoostStrength)))))

(event EventBeginPlay
  (bind _asplayer_controller (Utilities|Casting|CastToPlayerController (Pawn|GetController)))
  (Input|AddMappingContext (PlayerController|LocalPlayerSubsystems|GetEnhancedInputLocalPlayerSubsystem _asplayer_controller) "/Game/SkippyStone/Input/IM_SkippyStone.IM_SkippyStone" 0 "(bIgnoreAllPressedKeysUntilRelease=True,bForceImmediately=False,bNotifyUserSettings=False)")
  (Physics|AddImpulse (Variables|Default|GetMesh) (Variables|Default|GetStartImpulse) "None" true))

(event Collision|EventActorBeginOverlap
  (params (OtherActor :type Actor%20Object%20Reference)))

(event EventTick
  (params (DeltaSeconds :type Float%20%28single-precision%29))
  (bind _distancebelow (CallFunction|GetDistancetoSurface false))
  (CallFunction|UpdateBoostingState))

(fn ConstructionScript)

(fn GetDistancetoSurface
  (params (bDrawDebug :type Boolean))
  (bind _mesh (Variables|Default|GetMesh))
  (bind _returnvalue (Transformation|GetWorldLocation _mesh))
  (bind (_outhit _returnvalue_2) (Class|KismetSystemLibrary|SphereTraceSinglebyProfile _returnvalue (+ _returnvalue "0.000000,0.000000,-1000.000000") (* (.x (Variables|/Script/Engine.SceneComponent|GetRelativeScale3D _mesh)) 1e+02) "Water:Passthrough" false 0 (select bDrawDebug "ForDuration" "None") true))
  (if _returnvalue_2
    (Development|PrintString (Utilities|String|ToString(Float) (.Distance (Collision|BreakHitResult _outhit))) true true "(R=0.056400,G=1.000000,B=0.164249,A=1.000000)" 2.0 "distance")
    (else
      (Development|PrintString "no hit" true true "(R=1.000000,G=0.056642,B=0.144326,A=1.000000)" 2.0 "distance")))
  (return (.Distance (Collision|BreakHitResult _outhit))))

(fn Boost
  (params (DistanceToSurface :type Float%20%28double-precision%29) (ForwardBoostStrength :type Float%20%28double-precision%29) (UpBoostStrength :type Float%20%28double-precision%29))
  (bind _returnvalue (Math|Float|Clamp(Float) DistanceToSurface 0.0 1e+02))
  (bind _returnvalue_2 (Math|Vector|MakeVector ForwardBoostStrength 0.0 UpBoostStrength))
  (bind _mesh (Variables|Default|GetMesh))
  (bind _booststrengthcurve (Variables|Default|GetBoostStrengthCurve))
  (bind _returnvalue_3 (Math|Curves|GetFloatValue _booststrengthcurve _returnvalue))
  (bind _returnvalue_4 (* _returnvalue_3 _returnvalue_2))
  (bind (_x _y _z) (Math|Vector|BreakVector _returnvalue_4))
  (Variables|Default|SetisBoosting true)
  (bind _returnvalue_5 (Physics|GetPhysicsLinearVelocity _mesh "None"))
  (Physics|SetPhysicsLinearVelocity _mesh (Math|Vector|MakeVector (+ (.x _returnvalue_5) _x) (.y _returnvalue_5) _z) false "None")
  (return))

(fn UpdateBoostingState
  (bind _returnvalue (Physics|GetPhysicsLinearVelocity (Variables|Default|GetMesh) "None"))
  (Variables|Default|SetisBoosting (> (.z _returnvalue) 1e+02))
  (return))

(fn GetHeight
  (bind _distancebelow (CallFunction|GetDistancetoSurface false))
  (return _distancebelow))